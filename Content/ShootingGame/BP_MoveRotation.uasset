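; BP_MoveRotation is a shooting-game Blueprint that spins its Sphere component while IsPlay is true.
; On BeginPlay it binds to the DoPlay dispatcher of SwitchRef to start the spin, while the EventOverlap function sets IsPlay from IsBegin.
; Tick adds a fixed relative rotation each frame without delta-time scaling, so speed depends on frame rate.
; A looping Timeline for moving the Sphere is present but never runs.
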(event `self.ReceiveBeginPlay`
  (add `/Game/ShootingGame/BP_Switch.EventDispatcher_DoPlay` (`self.SwitchRef`) (`|CreateDelegate` :!event `EventOverlap`)))

(event `self.ReceiveTick`
  (params (DeltaSeconds :type "Float (single-precision)"))
  (if (`self.IsPlay`)
    (`SceneComponent.K2_AddRelativeRotation` (`self.Sphere`) (struct :`Yaw` 1.0) false false)))

(event `DoPlay`
  (set `self.IsPlay` true))

(fn `EventOverlap`
  (params (IsBegin :type Boolean))
  (set `self.IsPlay` IsBegin))

(fn `UserConstructionScript`)