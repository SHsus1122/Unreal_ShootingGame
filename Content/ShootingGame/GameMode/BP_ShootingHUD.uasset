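; BP_ShootingHUD is the shooting game's HUD, displaying the player's HP.
; On BeginPlay it creates the ShootingHudWidget, adds it to the viewport and binds to the UpdateHp dispatcher on player 0's BP_ShootingPlayerState.
; Binding retries on a short timer until the PlayerState cast succeeds, then pushes current HP with a hardcoded maximum.
; EventUpdateHp prints a debug string and passes HP values to the widget.
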(event `self.ReceiveBeginPlay`
  (bind _returnvalue (`|CreateWidget` "/Game/ShootingGame/Widget/ShootingHudWidget.ShootingHudWidget_C"))
  (bind _output_get (set `self.HudWidget` _returnvalue))
  (`UserWidget.AddToViewport` _output_get 0)
  (`self.BindByPlayerState`))

(fn `BindByPlayerState`
  (bind _asbp_shooting_player_state (cast `/Game/ShootingGame/GameMode/BP_ShootingPlayerState` (`Controller.PlayerState` (`GameplayStatics.GetPlayerController` 0)))
    (:`then`
      (add `/Game/ShootingGame/GameMode/BP_ShootingPlayerState.EventDispatcher_UpdateHp` _asbp_shooting_player_state (`|CreateDelegate` :!event `EventUpdateHp`))
      (`self.EventUpdateHp` (`/Game/ShootingGame/GameMode/BP_ShootingPlayerState.CurHp` _asbp_shooting_player_state) 100.0))
    (:`CastFailed`
      (`KismetSystemLibrary.K2_SetTimer` null "BindByPlayerState" 0.01))))

(fn `EventUpdateHp`
  (params (CurHp :type "Float (double-precision)") (MasxHp :type "Float (double-precision)"))
  (`KismetSystemLibrary.PrintString` (`KismetStringLibrary.Concat_StrStr` "HUD Update Hp - " (`KismetStringLibrary.Conv_DoubleToString` CurHp)) true true (struct :`G` 0.66 :`B` 1.0 :`A` 1.0) 60.0)
  (`/Game/ShootingGame/Widget/ShootingHudWidget.SetHp` (`self.HudWidget`) CurHp MasxHp))

(fn `UserConstructionScript`)